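; BP_Enemy4 is a kamikaze enemy that explodes on contact with an ally.
; When its capsule begins overlapping a static mesh component on a BP_BaseAlly, it applies its kamikaze damage to that ally.
; It then spawns a scaled-down Niagara explosion at its location and destroys itself.
; The construction script only calls its parent, and the other default events are unused.
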(event `self.Capsule.OnComponentBeginOverlap`
  (params (OverlappedComponent :type "PrimitiveComponent Object Reference") (OtherActor :type "Actor Object Reference") (OtherComp :type "PrimitiveComponent Object Reference") (OtherBodyIndex :type Integer) (bFromSweep :type Boolean) (SweepResult :type "HitResult Structure (by ref)"))
  (if (and (`GameplayStatics.ObjectIsA` OtherActor "/Game/Characters/Allies/BP_BaseAlly.BP_BaseAlly_C") (`GameplayStatics.ObjectIsA` OtherComp "/Script/Engine.StaticMeshComponent"))
    (bind _asbp_base_ally (cast `/Game/Characters/Allies/BP_BaseAlly` OtherActor))
    (`/Game/Characters/Allies/BP_BaseAlly.ApplyAllyDamage` _asbp_base_ally (`self.KamikazeDamageAmount`))
    (`NiagaraFunctionLibrary.SpawnSystemAtLocation` "/Game/MsvFx_Niagara_Explosion_Pack_01/Prefabs/Niagara_Explosion_02.Niagara_Explosion_02" (`SceneComponent.K2_GetComponentLocation` (`self.Scene`)) (struct) (0.8 0.8 0.8))
    (`self.K2_DestroyActor`)))

(fn `UserConstructionScript`
  (`parent.UserConstructionScript`))