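; BP_EnemyBase is an enemy base Blueprint that handles taking damage and paying out a money reward on death.
; ApplyEnemyDamage subtracts from Health and writes the Health/MaxHealth ratio into the WB_HealthBar widget, stopping early if that cast fails.
; At zero health or below, it adds DeathReward to Money on the first top-level WBP_IngameUI found by a widget search, then destroys the actor.
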(event `ApplyEnemyDamage`
  (params (DamageAmount :type "Float (double-precision)"))
  (set `self.Health` (- (`self.Health`) DamageAmount))
  (bind _aswb_health_bar (cast `/Game/Blueprints/UI/EnemyAndAlly/WB_HealthBar` (`WidgetComponent.GetWidget` (`self.HealthBar`))))
  (set `/Game/Blueprints/UI/EnemyAndAlly/WB_HealthBar.HealthPercent` (/ (`self.Health`) (`self.MaxHealth`)) _aswb_health_bar)
  (if (<= (`self.Health`) 0.0)
    (bind _foundwidgets (`WidgetBlueprintLibrary.GetAllWidgetsOfClass` "/Game/Blueprints/UI/Ingame/WBP_IngameUI.WBP_IngameUI_C"))
    (bind _output (`|GetArrayItem` _foundwidgets))
    (set `/Game/Blueprints/UI/Ingame/WBP_IngameUI.Money` (+ (`/Game/Blueprints/UI/Ingame/WBP_IngameUI.Money` _output) (`self.DeathReward`)) _output)
    (`self.K2_DestroyActor`)))

(fn `UserConstructionScript`)