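; Enemy wave manager that spawns a new wave every 20 seconds after play begins, indefinitely.
; Each wave randomly uses one of three preset combinations or one built from the shuffled enemy array, spawning at twelve scene-component points by index.
; It then increments the wave count and writes it to the in-game UI widget.
; GetEnemyCount, meant to size random waves, has its wave-scaled random Select left unconnected.
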(event `self.ReceiveBeginPlay`
  (`KismetSystemLibrary.Delay` 0.2)
  (set `self.SpawnLocations` (`|MakeArray` (`self.Scene1`) (`self.Scene2`) (`self.Scene3`) (`self.Scene4`) (`self.Scene5`) (`self.Scene6`) (`self.Scene7`) (`self.Scene8`) (`self.Scene9`) (`self.Scene10`) (`self.Scene11`) (`self.Scene12`)))
  (`self.NextWave`))

(event `NextWave`
  (`KismetArrayLibrary.Array_Clear` (`self.CombinationRandom`))
  (set `self.EnemyCount` (`self.GetEnemyCount`))
  (`KismetArrayLibrary.Array_Shuffle` (`self.EnnemyArray`))
  (for _index (range (+ (`self.EnemyCount`) 1))
    (`KismetArrayLibrary.Array_Add` (`self.CombinationRandom`) (`|GetArrayItem` (`self.EnnemyArray`) _index)))
  (for (_array_element _array_index) (select `int` (`KismetMathLibrary.RandomIntegerInRange` 0 3) :`0` (`self.Combination1`) :`1` (`self.Combination2`) :`2` (`self.Combination3`) :`3` (`self.CombinationRandom`))
    (`|SpawnActorFromClass` _array_element (`SceneComponent.K2_GetComponentToWorld` (`|GetArrayItem` (`self.SpawnLocations`) _array_index)) "AdjustIfPossibleButAlwaysSpawn" "MultiplyWithRoot" null null))
  (set `self.WaveCount` (+ (`self.WaveCount`) 1))
  (bind _foundwidgets (`WidgetBlueprintLibrary.GetAllWidgetsOfClass` "/Game/Blueprints/UI/Ingame/WBP_IngameUI.WBP_IngameUI_C"))
  (set `/Game/Blueprints/UI/Ingame/WBP_IngameUI.WaveCount` (`self.WaveCount`) (`|GetArrayItem` _foundwidgets))
  (`KismetSystemLibrary.Delay` 20.0)
  (`self.NextWave`))

(fn `UserConstructionScript`)