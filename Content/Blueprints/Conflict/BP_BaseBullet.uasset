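; BP_BaseBullet is a homing projectile that deals damage for either the enemy or allied side.
; From BeginPlay, a timeline lerps its current location toward a target component's live location, scaled by AmmoSpeed, destroying it if that target becomes invalid.
; On sphere overlap, the Enemy flag selects which opposing base class counts as a hit.
; A hit applies AmmoStrength damage to the stored attack target, not the overlapped actor, then destroys the bullet.
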(event `self.ReceiveBeginPlay`
  (bind (_direction _newtrack_3) (`Timeline|Timeline` :!via `PlayFromStart`)
    (:`Update`
      (`/Engine/EditorBlueprintResources/StandardMacros.IsValid` (`self.TargetForEndLocation`)
        (:`Is Valid`
          (`self.K2_SetActorLocation` (`KismetMathLibrary.VLerp` (`self.K2_GetActorLocation`) (`SceneComponent.K2_GetComponentLocation` (`self.TargetForEndLocation`)) (* _newtrack_3 (`self.AmmoSpeed`)))))
        (:`Is Not Valid`
          (`self.K2_DestroyActor`))))))

(event `self.Sphere.OnComponentBeginOverlap`
  (params (OverlappedComponent :type "PrimitiveComponent Object Reference") (OtherActor :type "Actor Object Reference") (OtherComp :type "PrimitiveComponent Object Reference") (OtherBodyIndex :type Integer) (bFromSweep :type Boolean) (SweepResult :type "HitResult Structure (by ref)"))
  (bind _returnvalue (`GameplayStatics.ObjectIsA` OverlappedComponent "/Script/Engine.SphereComponent"))
  (if (`self.Enemy`)
    (if (and _returnvalue (`GameplayStatics.ObjectIsA` OtherActor "/Game/Characters/Allies/BP_BaseAlly.BP_BaseAlly_C"))
      (`/Game/Characters/Allies/BP_BaseAlly.ApplyAllyDamage` (`self.AttackTargetActorAlly`) (`self.AmmoStrength`))
      (`self.K2_DestroyActor`))
    (elif (and _returnvalue (`GameplayStatics.ObjectIsA` OtherActor "/Game/Characters/Enemies/Blueprints/BP_EnemyBase.BP_EnemyBase_C"))
      (`/Game/Characters/Enemies/Blueprints/BP_EnemyBase.ApplyEnemyDamage` (`self.AttackTargetActorEnemy`) (`self.AmmoStrength`))
      (`self.K2_DestroyActor`))))

(fn `UserConstructionScript`)